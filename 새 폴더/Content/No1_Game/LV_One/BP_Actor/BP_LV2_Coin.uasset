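; Collectible coin actor that spins and bobs up and down until something overlaps it.
; A looping 0.01-second timer, rather than Tick, drives UpdateCoinMove, which yaws the mesh and moves it between two relative heights, flipping IsRight at each limit.
; On any mesh overlap, with no filter on the other actor, it hides itself, fires the Hidden event dispatcher and disables collision instead of being destroyed.
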(event OnComponentBeginOverlap(StaticMesh)
  (params (OverlappedComponent :type Primitive%20Component%20Object%20Reference) (OtherActor :type Actor%20Object%20Reference) (OtherComp :type Primitive%20Component%20Object%20Reference) (OtherBodyIndex :type Integer) (bFromSweep :type Boolean) (SweepResult :type Hit%20Result%20Structure%20%28by%20ref%29))
  (Development|PrintString "Begin Overlap Coin!!!")
  (Rendering|SetActorHiddenInGame true)
  (Default|CallEventDispatcherHidden)
  (Collision|SetCollisionEnabled (Variables|Default|GetStaticMesh) "NoCollision"))

(event EventBeginPlay
  (Utilities|Time|SetTimerbyFunctionName 0 "UpdateCoinMove" 0.01 true))

(fn ConstructionScript)

(fn UpdateRotaion
  (params (DeltaSeconds :type Float%20%28single-precision%29))
  (Transformation|AddRelativeRotation (Variables|Default|GetStaticMesh) (Math|Rotator|MakeRotator 0.0 0.0 (* DeltaSeconds 1.8e+02)) false false))

(fn UpdateMoveUpDown
  (params (Delta%20Seconds :type Float%20%28single-precision%29))
  (bind _speed (Variables|Default|GetSpeed))
  (bind _staticmesh (Variables|Default|GetStaticMesh))
  (bind _returnvalue (* Delta%20Seconds _speed))
  (if (Variables|Default|GetIsRight)
    (Transformation|AddRelativeLocation _staticmesh (Math|Vector|MakeVector 0.0 0.0 _returnvalue) false false)
    (if (> (.z (Variables|/Script/Engine.SceneComponent|GetRelativeLocation (Variables|Default|GetStaticMesh))) 1.5e+02)
      (Variables|Default|SetIsRight false))
    (else
      (bind _result (Math|Float|NegateFloat _returnvalue)
        (:%20%20
          (Transformation|AddRelativeLocation _staticmesh (Math|Vector|MakeVector 0.0 0.0 _result) false false)
          (if (< (.z (Variables|/Script/Engine.SceneComponent|GetRelativeLocation (Variables|Default|GetStaticMesh))) 5e+01)
            (Variables|Default|SetIsRight true)))))))

(fn UpdateCoinMove
  (Utilities|FlowControl|Sequence
    (:then_0
      ;[1 1 1] 회전 업데이트
      (CallFunction|UpdateRotaion 0.01))
    (:then_1
      ;[1 1 1] 위치 업데이트
      (CallFunction|UpdateMoveUpDown 0.01))))