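; Game mode for Stage 1 of No1_Game that tracks ruby pickups and shows the count on the HUD.
; On BeginPlay it pushes the LV1_Instance game instance's ruby score and total to BP_LV1_HUD, then calls RubySaveGame on the instance.
; The RubyScore function passes the incremented score to the instance's Ruby function, with a zero total argument, and refreshes the HUD counter.
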(event EventBeginPlay
  (bind _aslv1_instance (Utilities|Casting|CastToLV1_Instance (Game|GetGameInstance)))
  (bind _asbp_lv1_hud (Utilities|Casting|CastToBP_LV1_HUD (HUD|GetHUD (Game|GetPlayerController 0))))
  (Default|SetRubyCount _asbp_lv1_hud (Variables|/Game/No1_Game/LV1_Instance.LV1_Instance_C|GetRubyScore _aslv1_instance) (Variables|/Game/No1_Game/LV1_Instance.LV1_Instance_C|GetRubyTotal _aslv1_instance))
  (Default|RubySaveGame _aslv1_instance))

(fn ConstructionScript)

(fn RubyScore
  (bind _aslv1_instance (Utilities|Casting|CastToLV1_Instance (Game|GetGameInstance)))
  (Default|Ruby _aslv1_instance (+ (Variables|/Game/No1_Game/LV1_Instance.LV1_Instance_C|GetRubyScore _aslv1_instance) 1))
  (bind _asbp_lv1_hud (Utilities|Casting|CastToBP_LV1_HUD (HUD|GetHUD (Game|GetPlayerController 0))))
  (Default|SetRubyCount _asbp_lv1_hud (Variables|/Game/No1_Game/LV1_Instance.LV1_Instance_C|GetRubyScore _aslv1_instance) (Variables|Default|GetRubyTotal)))