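; BP_LV1_HUD is the Level 1 HUD Blueprint that creates the LV1_Widget on BeginPlay, adds it to the viewport and shows the ruby count.
; SetRubyCount passes score and total to the widget's SetRuby.
; If the widget is not yet valid, it stores both values and BackUPRuby retries on a short timer until the widget exists, covering calls that arrive before BeginPlay creates it.
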(event EventBeginPlay
  (bind _returnvalue (UserInterface|CreateWidget "/Game/No1_Game/Stage1/GameMode/LV1_Widget.LV1_Widget_C"))
  (bind _output_get (Variables|Default|SetLV1Widget _returnvalue))
  (UserInterface|Viewport|AddtoViewport _output_get 0))

(event Collision|EventActorBeginOverlap
  (params (OtherActor :type Actor%20Object%20Reference)))

(event EventTick
  (params (DeltaSeconds :type Float%20%28single-precision%29)))

(fn ConstructionScript)

(fn SetRubyCount
  (params (Score :type Integer) (Total :type Integer))
  (bind _lv1widget (Variables|Default|GetLV1Widget))
  (Utilities|IsValid _lv1widget
    (:Is%20Valid
      (Default|SetRuby _lv1widget Score Total))
    (:Is%20Not%20Valid
      (Variables|Default|SetBackUPScore Score)
      (Variables|Default|SetBackUPTaotal Total)
      (Utilities|Time|SetTimerbyFunctionName 0 "BackUPRuby" 0.1))))

(fn BackUPRuby
  (bind _lv1widget (Variables|Default|GetLV1Widget))
  (Utilities|IsValid _lv1widget
    (:Is%20Valid
      (Default|SetRuby _lv1widget (Variables|Default|GetBackUPScore) (Variables|Default|GetBackUPTaotal)))
    (:Is%20Not%20Valid
      (Utilities|Time|SetTimerbyFunctionName 0 "BackUPRuby" 0.1))))