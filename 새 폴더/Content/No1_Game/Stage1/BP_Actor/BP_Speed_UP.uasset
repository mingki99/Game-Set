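; Speed boost pickup for Stage 1 that triggers when an LV1Game_Charater overlaps its capsule, then hides itself and disables its collision.
; It doubles the player's max walk speed, calls the character's Run, and halves the speed again after a timer.
; Looping name-based timers repeatedly spawn NI_SpeedUP effect actors near the player mesh and periodically hide all of them without destroying them, until separate timers clear both loops.
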(event OnComponentBeginOverlap(Capsule)
  (params (OverlappedComponent :type Primitive%20Component%20Object%20Reference) (OtherActor :type Actor%20Object%20Reference) (OtherComp :type Primitive%20Component%20Object%20Reference) (OtherBodyIndex :type Integer) (bFromSweep :type Boolean) (SweepResult :type Hit%20Result%20Structure%20%28by%20ref%29))
  (Utilities|Casting|CastToLV1Game_Charater OtherActor)
  (Rendering|SetActorHiddenInGame true)
  (Collision|SetCollisionEnabled (Variables|Default|GetCapsule) "NoCollision")
  (CallFunction|SpeedUP)
  (Utilities|Time|SetTimerbyFunctionName 0 "SpeedDown" 3.5)
  (bind _aslv1game_charater (Utilities|Casting|CastToLV1Game_Charater (Game|Player|GetPlayerPawn 0)))
  (Default|Run _aslv1game_charater)
  (CallFunction|NiagaraProscces))

(fn ConstructionScript)

(fn SpeedUP
  (bind _aslv1game_charater (Utilities|Casting|CastToLV1Game_Charater (Game|Player|GetPlayerPawn 0)))
  (Variables|/Script/Engine.CharacterMovementComponent|SetMaxWalkSpeed (Variables|/Script/Engine.Character|GetCharacterMovement _aslv1game_charater) (* (Class|MovementComponent|GetMaxSpeed (Variables|/Script/Engine.Character|GetCharacterMovement _aslv1game_charater)) 2.0)))

(fn SpeedDown
  (bind _aslv1game_charater (Utilities|Casting|CastToLV1Game_Charater (Game|Player|GetPlayerPawn 0)))
  (bind _output_get (Variables|Default|SetCahrSpeed (Class|MovementComponent|GetMaxSpeed (Variables|/Script/Engine.Character|GetCharacterMovement _aslv1game_charater))))
  (Variables|/Script/Engine.CharacterMovementComponent|SetMaxWalkSpeed (Variables|/Script/Engine.Character|GetCharacterMovement _aslv1game_charater) (/ _output_get 2.0)))

(fn NiagaraPrticle
  (bind _aslv1game_charater (Utilities|Casting|CastToLV1Game_Charater (Game|Player|GetPlayerPawn 0)))
  (Game|SpawnActorfromClass "/Game/No1_Game/Stage1/BP_Actor/Particle/NI_SpeedUP.NI_SpeedUP_C" (Math|Transform|MakeTransform (+ (.location (Transformation|GetWorldTransform (Variables|/Script/Engine.Character|GetMesh _aslv1game_charater))) "0.000000,100.000000, 0") (.rotation (Transformation|GetWorldTransform (Variables|/Script/Engine.Character|GetMesh _aslv1game_charater))) "1,1,1") "Undefined" 0 0))

(fn NiataraHidden
  (bind _outactors (Actor|GetAllActorsOfClass "/Game/No1_Game/Stage1/BP_Actor/Particle/NI_SpeedUP.NI_SpeedUP_C"))
  (bind _output_get (Variables|Default|SetOut%20Actors _outactors))
  (for _array_element _output_get
    (Rendering|SetVisibility (Variables|/Game/No1_Game/Stage1/BP_Actor/Particle/NI_SpeedUP.NI_SpeedUP_C|GetNiagara _array_element) false false)
    (Collision|SetCollisionEnabled (Variables|/Game/No1_Game/Stage1/BP_Actor/Particle/NI_SpeedUP.NI_SpeedUP_C|GetNiagara _array_element) "NoCollision")))

(fn TiemerNIargaraHiddenClear
  (Utilities|Time|ClearTimerbyFunctionName 0 "NiataraHidden"))

(fn TimerNIagaraSpawnClear
  (Utilities|Time|ClearTimerbyFunctionName 0 "NiagaraPrticle"))

(fn NiagaraProscces
  (Utilities|Time|SetTimerbyFunctionName 0 "NiagaraPrticle" 0.05 true)
  (Utilities|Time|SetTimerbyFunctionName 0 "TimerNIagaraSpawnClear" 3.5)
  (Utilities|Time|SetTimerbyFunctionName 0 "NiataraHidden" 1.0 true)
  (Utilities|Time|SetTimerbyFunctionName 0 "TiemerNIargaraHiddenClear" 5.0))