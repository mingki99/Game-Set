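; Stage 1 cannon actor that tracks the player and periodically fires physics balls at them.
; On Tick its Arrow component smoothly rotates toward player pawn 0 using a look-at rotation lerp.
; DoShoot runs at BeginPlay and on a looping timer, spawning an LV1_Ball at the Arrow's transform.
; Each ball has its velocity zeroed, then receives a strong forward impulse on its Sphere.
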(event EventBeginPlay
  (Variables|Default|SetTarget (Game|Player|GetPlayerPawn 0))
  (CallFunction|DoShoot)
  (Utilities|Time|SetTimerbyFunctionName 0 "DoShoot" 5.0 true))

(event EventTick
  (params (DeltaSeconds :type Float%20%28single-precision%29))
  (bind _arrow (Variables|Default|GetArrow))
  (Transformation|SetWorldRotation _arrow (Math|Rotator|Lerp(Rotator) (Transformation|GetWorldRotation _arrow) (Math|Rotator|FindLookatRotation (Transformation|GetWorldLocation _arrow) (Transformation|GetActorLocation (Variables|Default|GetTarget))) 0.1 true) false false))

(fn ConstructionScript)

(fn DoShoot
  (bind _arrow (Variables|Default|GetArrow))
  (bind _returnvalue (Game|SpawnActorfromClass "/Game/No1_Game/Stage1/BP_Actor/LV1_Ball.LV1_Ball_C" (Math|Transform|MakeTransform (Transformation|GetWorldLocation _arrow) (Transformation|GetWorldRotation _arrow) "1,1,1") "Undefined" 0 0))
  (Class|PrimitiveComponent|SetAllPhysicsLinearVelocity (Variables|/Game/No1_Game/Stage1/BP_Actor/LV1_Ball.LV1_Ball_C|GetSphere _returnvalue) "0, 0, 0" false)
  (Physics|AddImpulse (Variables|/Game/No1_Game/Stage1/BP_Actor/LV1_Ball.LV1_Ball_C|GetSphere _returnvalue) (* (Math|Vector|GetForwardVector (Variables|/Game/No1_Game/Stage1/BP_Actor/LV1_Ball.LV1_Ball_C|GetSphere _returnvalue)) 5e+05) "None" false))