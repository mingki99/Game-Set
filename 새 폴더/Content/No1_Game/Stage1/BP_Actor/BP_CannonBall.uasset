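; BP_CannonBall is a cannon hazard that fires a physics ball toward the player's pawn.
; Its Arrow smoothly rotates toward the player each tick, while a looping timer calls DoShoot to reset and relaunch the same ball from the Arrow.
; Hitting a BP_SwatCharacter triggers ragdoll, a strong knockback impulse, an explosion effect and sound.
; An unused spawn-based firing path remains disconnected.
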(event OnComponentHit(CannonBall)
  (params (HitComponent :type Primitive%20Component%20Object%20Reference) (OtherActor :type Actor%20Object%20Reference) (OtherComp :type Primitive%20Component%20Object%20Reference) (NormalImpulse :type Vector :default "0, 0, 0") (Hit :type Hit%20Result%20Structure%20%28by%20ref%29))
  (bind _cannonball (Variables|Default|GetCannonBall))
  (bind _returnvalue (Transformation|GetWorldLocation _cannonball))
  (Development|PrintString (Utilities|GetDisplayName OtherActor))
  (bind _asbp_swat_character (Utilities|Casting|CastToBP_SwatCharacter OtherActor))
  (Default|DoRagdoll _asbp_swat_character)
  (Physics|AddImpulse (Variables|/Script/Engine.Character|GetMesh _asbp_swat_character) (* (Math|Vector|GetForwardVector (Math|Rotator|FindLookatRotation _returnvalue (Transformation|GetActorLocation _asbp_swat_character))) 1e+07) "None" false)
  (Effects|SpawnEmitteratLocation "/Game/StarterContent/Particles/P_Explosion.P_Explosion" _returnvalue)
  (Audio|Components|Audio|Play (Variables|Default|GetExplosion_Cue) 0.0))

(event EventBeginPlay
  (Variables|Default|SetTarget (Game|Player|GetPlayerPawn 0))
  (CallFunction|DoShoot)
  (Utilities|Time|SetTimerbyFunctionName 0 "DoShoot" 5.0 true))

(event EventTick
  (params (DeltaSeconds :type Float%20%28single-precision%29))
  (bind _arrow (Variables|Default|GetArrow))
  (Transformation|SetWorldRotation _arrow (Math|Rotator|Lerp(Rotator) (Transformation|GetWorldRotation _arrow) (Math|Rotator|FindLookatRotation (Transformation|GetWorldLocation _arrow) (Transformation|GetActorLocation (Variables|Default|GetTarget))) 0.1 true) false false))

(fn ConstructionScript)

(fn DoShoot
  (bind _arrow (Variables|Default|GetArrow))
  (bind _cannonball (Variables|Default|GetCannonBall))
  (Transformation|SetWorldLocationAndRotation (Variables|Default|GetCannonBall) (Transformation|GetWorldLocation _arrow) (Transformation|GetWorldRotation _arrow) false false)
  (Class|PrimitiveComponent|SetAllPhysicsLinearVelocity _cannonball "0, 0, 0" false)
  (Physics|AddImpulse _cannonball (* (Math|Vector|GetForwardVector _cannonball) 5e+05) "None" false))