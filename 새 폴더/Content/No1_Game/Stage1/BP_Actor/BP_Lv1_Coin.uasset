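; Collectible coin for Stage 1 that bobs vertically and is picked up when the level 1 player character touches it.
; A fast looping timer runs CoinMove, shifting the capsule up and down at a Speed-scaled rate, flipping IsRight at the height limits.
; On pickup it hides itself, calls the LV1 coin event dispatcher, disables capsule collision and spawns a Niagara burst instead of being destroyed.
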(event OnComponentBeginOverlap(Capsule)
  (params (OverlappedComponent :type Primitive%20Component%20Object%20Reference) (OtherActor :type Actor%20Object%20Reference) (OtherComp :type Primitive%20Component%20Object%20Reference) (OtherBodyIndex :type Integer) (bFromSweep :type Boolean) (SweepResult :type Hit%20Result%20Structure%20%28by%20ref%29))
  (bind _capsule (Variables|Default|GetCapsule))
  (bind _returnvalue (Transformation|GetWorldTransform _capsule))
  (Utilities|Casting|CastToLV1Game_Charater OtherActor)
  (Rendering|SetActorHiddenInGame true)
  (Default|CallLV1CoinEventDispatcher)
  (Collision|SetCollisionEnabled (Variables|Default|GetCapsule) "NoCollision")
  (Niagara|SpawnSystematLocation "/Game/No1_Game/Stage1/BP_Actor/Particle/Nieagara/NO1_NiagaraSystems/NS_CoinBurst2.NS_CoinBurst2" (.location _returnvalue) (.rotation _returnvalue) "25.000000,25.000000,25.000000"))

(event EventBeginPlay
  (Utilities|Time|SetTimerbyFunctionName 0 "CoinMove" 0.01 true))

(fn ConstructionScript)

(fn CoinMove
  (bind _capsule (Variables|Default|GetCapsule))
  (bind _speed (Variables|Default|GetSpeed))
  (bind _returnvalue (* 0.01 _speed))
  (if (Variables|Default|GetIsRight)
    (Transformation|AddRelativeLocation _capsule (Math|Vector|MakeVector 0.0 0.0 _returnvalue) false false)
    (if (> (.z (Variables|/Script/Engine.SceneComponent|GetRelativeLocation (Variables|Default|GetCapsule))) 1e+02)
      (Variables|Default|SetIsRight false))
    (else
      (bind _result (Math|Float|NegateFloat _returnvalue)
        (:%20%20
          (Transformation|AddRelativeLocation _capsule (Math|Vector|MakeVector 0.0 0.0 _result) false false)
          (if (< (.z (Variables|/Script/Engine.SceneComponent|GetRelativeLocation (Variables|Default|GetCapsule))) 5e+01)
            (Variables|Default|SetIsRight true)))))))