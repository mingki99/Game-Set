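; BP_SlowChar is a one-shot slow trap actor for Stage 1 that reacts when the player character overlaps its Plane.
; On overlap by LV1Game_Charater, it calls ISeeYou on every BP_LV1Villain, alerting them.
; SlowSpeed runs inside that same loop, so each villain divides the character's MaxWalkSpeed again, with no restore here.
; SlowSpeed also disables the Plane's collision, preventing retriggers.
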(event OnComponentBeginOverlap(Plane)
  (params (OverlappedComponent :type Primitive%20Component%20Object%20Reference) (OtherActor :type Actor%20Object%20Reference) (OtherComp :type Primitive%20Component%20Object%20Reference) (OtherBodyIndex :type Integer) (bFromSweep :type Boolean) (SweepResult :type Hit%20Result%20Structure%20%28by%20ref%29))
  (bind _aslv1game_charater (Utilities|Casting|CastToLV1Game_Charater OtherActor))
  (bind _outactors (Actor|GetAllActorsOfClass "/Game/No1_Game/CharAnim/BP_LV1Villain.BP_LV1Villain_C"))
  (bind _output_get (Variables|Default|SetOut%20Actors _outactors))
  (for _array_element _output_get
    (Default|ISeeYou _array_element)
    (CallFunction|SlowSpeed _aslv1game_charater)))

(event EventBeginPlay)

(event Collision|EventActorBeginOverlap
  (params (OtherActor :type Actor%20Object%20Reference)))

(event EventTick
  (params (DeltaSeconds :type Float%20%28single-precision%29)))

(fn ConstructionScript)

(fn SlowSpeed
  (params (타깃 :type Character%20Object%20Reference))
  (bind _charactermovement (Variables|/Script/Engine.Character|GetCharacterMovement 타깃))
  (Variables|/Script/Engine.CharacterMovementComponent|SetMaxWalkSpeed _charactermovement (/ (Variables|/Script/Engine.CharacterMovementComponent|GetMaxWalkSpeed _charactermovement) 1.5))
  (Collision|SetCollisionEnabled (Variables|Default|GetPlane) "NoCollision"))