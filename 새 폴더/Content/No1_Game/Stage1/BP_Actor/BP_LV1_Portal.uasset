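; Level 1 portal actor that opens the level named by LevelName when the player character overlaps its capsule, with no coin check.
; On BeginPlay it binds to each coin's event dispatcher and sets the HUD ruby count from hidden versus total coins.
; OnHiddenCheck adds score through the game mode's RubyScore.
; CheckCoin tests whether all coins are hidden but is not called here, and an instance-based HUD-and-save chain is disconnected.
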(event OnComponentBeginOverlap(Capsule)
  (params (OverlappedComponent :type Primitive%20Component%20Object%20Reference) (OtherActor :type Actor%20Object%20Reference) (OtherComp :type Primitive%20Component%20Object%20Reference) (OtherBodyIndex :type Integer) (bFromSweep :type Boolean) (SweepResult :type Hit%20Result%20Structure%20%28by%20ref%29))
  (Utilities|Casting|CastToLV1Game_Charater OtherActor)
  (Game|OpenLevel(byName) (Variables|Default|GetLevel%20Name)))

(event EventBeginPlay
  (bind (_curcount _maxcount) (CallFunction|GetHiddenCoinCount))
  (Utilities|FlowControl|Sequence
    (:then_0
      (bind _outactors (Actor|GetAllActorsOfClass "/Game/No1_Game/Stage1/BP_Actor/BP_Lv1_Coin.BP_Lv1_Coin_C"))
      (bind _output_get (Variables|Default|SetOut%20Actors _outactors))
      (for _array_element _output_get
        (EventDispatchers|BindEventtoLV1CoinEventDispatcher _array_element (EventDispatchers|CreateEvent :!event OnHiddenCheck))))
    (:then_1
      (bind _asbp_lv1_hud (Utilities|Casting|CastToBP_LV1_HUD (HUD|GetHUD (Game|GetPlayerController 0))))
      (Default|SetRubyCount _asbp_lv1_hud _curcount _maxcount))))

(fn ConstructionScript)

(fn CheckCoin
  (for _array_element 0
    (if (not (Variables|/Script/Engine.Actor|GetbHidden _array_element))
      (return false)))
  (return true))

(fn OnHiddenCheck
  ;[1 1 1] 점수 증가
  (bind _asbp_no_1game_mode (Utilities|Casting|CastToBP_No1GameMode (Game|GetGameMode)))
  (Default|RubyScore _asbp_no_1game_mode))

(fn GetHiddenCoinCount
  (bind _out_actors (Variables|Default|GetOut%20Actors))
  (for _array_element _out_actors
    (if (Variables|/Script/Engine.Actor|GetbHidden _array_element)
      (Math|Integer|IncrementInt (LocalVariables|GetHiddenCount))))
  (return (LocalVariables|GetHiddenCount) (Utilities|Array|Length _out_actors)))