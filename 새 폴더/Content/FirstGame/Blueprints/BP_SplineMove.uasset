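; Spline mover actor that shuttles a cube back and forth along a spline, matching its location and rotation to the path.
; On BeginPlay, a looping short-interval timer calls the Forward,backward function, which steps the distance at a fixed speed and repositions the cube in local space.
; The IsForward flag flips whenever the distance passes either end of the spline.
; An alternative timeline-driven version remains in the event graph but is disconnected.
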(event EventBeginPlay
  (Utilities|Time|SetTimerbyFunctionName 0 "Forward,backward" 0.01 true))

(event Collision|EventActorBeginOverlap
  (params (OtherActor :type Actor%20Object%20Reference)))

(event EventTick
  (params (DeltaSeconds :type Float%20%28single-precision%29)))

(fn ConstructionScript)

(fn Forward,backward
  (bind _returnvalue (* 0.01 3e+02))
  (bind _spline (Variables|Default|GetSpline))
  (bind _cube (Variables|Default|GetCube))
  (bind _spline_2 (Variables|Default|GetSpline))
  (if (Variables|Default|GetIsForward)
    ;[1 1 1] Forward
    (bind _output_get (Variables|Default|SetDistance (+ _returnvalue (Variables|Default|GetDistance))))
    (Transformation|SetRelativeTransform _cube (Math|Transform|MakeTransform (Spline|GetLocationatDistanceAlongSpline _spline_2 _output_get "Local") (Spline|GetRotationatDistanceAlongSpline _spline_2 _output_get "Local") (Variables|/Script/Engine.SceneComponent|GetRelativeScale3D _cube)) false false)
    (if (> (Variables|Default|GetDistance) (Spline|GetSplineLength (Variables|Default|GetSpline)))
      (Variables|Default|SetIsForward false))
    (else
      ;[1 1 1] back
      (bind _output_get_2 (Variables|Default|SetDistance (- (Variables|Default|GetDistance) _returnvalue)))
      (Transformation|SetRelativeTransform (Variables|Default|GetCube) (Math|Transform|MakeTransform (Spline|GetLocationatDistanceAlongSpline _spline _output_get_2 "Local") (Spline|GetRotationatDistanceAlongSpline _spline _output_get_2 "Local") (Variables|/Script/Engine.SceneComponent|GetRelativeScale3D (Variables|Default|GetCube))) false false)
      (if (<= (Variables|Default|GetDistance) 0.0)
        (Variables|Default|SetIsForward true)))))