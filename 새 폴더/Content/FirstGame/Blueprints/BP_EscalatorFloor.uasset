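; Escalator floor step that travels along a spline and loops back to the start.
; A looping 0.01-second timer, used instead of Tick, advances a distance by Speed and snaps the actor to the spline transform there.
; Past the spline's end, it hides the cube, disables its collision and stops the movement timer.
; After a short delay, SetStartPoint returns the actor to the start, restores the cube and restarts movement.
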(event EventBeginPlay
  (Utilities|Time|SetTimerbyFunctionName 0 "UPdateMoveFloor" 0.01 true))

(event Collision|EventActorBeginOverlap
  (params (OtherActor :type Actor%20Object%20Reference)))

(event EventTick
  (params (DeltaSeconds :type Float%20%28single-precision%29)))

(fn ConstructionScript)

(fn UPdateMoveFloor
  (bind _cube (Variables|Default|GetCube))
  (bind _output_get (Variables|Default|SetDistance (+ (* 0.01 (Variables|Default|GetSpeed)) (Variables|Default|GetDistance))))
  (Transformation|SetActorTransform (Spline|GetTransformatDistanceAlongSpline (Variables|Default|Getspline) _output_get "World" false))
  (if (> (Variables|Default|GetDistance) (Spline|GetSplineLength (Variables|Default|Getspline)))
    (Rendering|SetVisibility _cube false false)
    (Collision|SetCollisionEnabled _cube "NoCollision")
    (Utilities|Time|SetTimerbyFunctionName 0 "SetStartPoint" 0.1)
    (Utilities|Time|ClearTimerbyFunctionName 0 "UPdateMoveFloor")))

(fn SetStartPoint
  (bind _cube (Variables|Default|GetCube))
  (bind _output_get (Variables|Default|SetDistance 0.0))
  (Transformation|SetActorTransform (Spline|GetTransformatDistanceAlongSpline (Variables|Default|Getspline) _output_get "World" false))
  (Rendering|SetVisibility _cube true false)
  (Collision|SetCollisionEnabled _cube "QueryAndPhysics")
  (Utilities|Time|SetTimerbyFunctionName 0 "UPdateMoveFloor" 0.01 true))